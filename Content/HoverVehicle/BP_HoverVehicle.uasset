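; Player-controlled hover vehicle with twin projectile guns and a weapon overheat system.
; W/S and Left/Right keys set force and torque values that Tick applies to the physics Cube for thrust and turning.
; Holding Space spawns projectiles from two spawn points, with a Delay in Tick pacing the shots.
; Shots build heat that drains each tick; overheating blocks firing until heat reaches zero, with dispatchers broadcasting state and percentage.
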(event `Key|W`
  (params (Key :type "Key Structure"))
  (:`Pressed`
    (set `self.Forward Force` 500000.0))
  (:`Released`
    (set `self.Forward Force` 0.0 :!label _label)))

(event `Key|Right`
  (params (Key :type "Key Structure"))
  (:`Pressed`
    (set `self.turn Torque` 400000000.0))
  (:`Released`
    (set `self.turn Torque` 0.0 :!label _label_2)))

(event `Key|S`
  (params (Key :type "Key Structure"))
  (:`Pressed`
    (set `self.Forward Force` -500000.0))
  (:`Released`
    (goto _label)))

(event `Key|Left`
  (params (Key :type "Key Structure"))
  (:`Pressed`
    (set `self.turn Torque` -400000000.0))
  (:`Released`
    (goto _label_2)))

(event `self.ReceiveTick`
  (params (DeltaSeconds :type "Float (single-precision)"))
  (`|ExecutionSequence`
    (:`then_0`
      (`PrimitiveComponent.AddForce` (`self.Cube`) (* (`self.GetActorForwardVector`) (`self.Forward Force`)) "None" false)
      (`PrimitiveComponent.AddTorqueInDegrees` (`self.Cube`) (* (`self.GetActorUpVector`) (`self.turn Torque`)) "None" false))
    (:`then_1`
      (if (and (`PlayerController.IsInputKeyDown` (`GameplayStatics.GetPlayerController` 0) "SpaceBar") (not (`self.WeaponOverheated`)))
        (`KismetSystemLibrary.Delay` 0.05)
        (`|SpawnActorFromClass` "/Game/HoverVehicle/HoverGunProjectiles.HoverGunProjectiles_C" (`SceneComponent.K2_GetComponentToWorld` (`self.bulletSpawn1`)) "Undefined" "OverrideRootScale" null null)
        (`|SpawnActorFromClass` "/Game/HoverVehicle/HoverGunProjectiles.HoverGunProjectiles_C" (`SceneComponent.K2_GetComponentToWorld` (`self.bulletSpawn2`)) "Undefined" "OverrideRootScale" null null)
        (`self.FireHeatBuildup`)))
    (:`then_2`
      (`self.ReduceHeatBuildup` DeltaSeconds))))

(event `Key|SpaceBar`
  (params (Key :type "Key Structure")))

(fn `FireHeatBuildup`
  (bind _returnvalue (+ (`self.HeatCurrent`) (`self.HeatBuildupRate`)))
  (if (>= _returnvalue (`self.HeatMax`))
    (set `self.HeatCurrent` (`self.HeatMax`))
    (bind _output_get (set `self.WeaponOverheated` true))
    (`self.WeaponOverheatedDispatcher` _output_get)
    (else
      (set `self.HeatCurrent` _returnvalue))))

(fn `ReduceHeatBuildup`
  (params (DeltaT :type "Float (double-precision)"))
  (bind _returnvalue (- (`self.HeatCurrent`) (* DeltaT (`self.HeatReductionRate`))))
  (`|ExecutionSequence`
    (:`then_0`
      (if (> (`self.HeatCurrent`) 0.0)
        (if (<= _returnvalue 0.0)
          (set `self.HeatCurrent` 0.0)
          (bind _output_get (set `self.WeaponOverheated` false))
          (`self.WeaponOverheatedDispatcher` _output_get)
          (else
            (set `self.HeatCurrent` _returnvalue)))))
    (:`then_1`
      (`self.WeaponOverheatPercentDispatcher` (/ (`self.HeatCurrent`) (`self.HeatMax`))))))

(fn `UserConstructionScript`)